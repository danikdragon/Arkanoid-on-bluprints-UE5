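; BP_movementBall is a ball actor that moves itself every tick and bounces off whatever it hits.
; Each tick it lowers its speed by a fixed step while above a minimum, then does a swept world offset along its direction vector.
; On a blocking hit, the direction is reflected around the surface normal, giving simple bounces without physics simulation.
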(event `self.ReceiveTick`
  (params (DeltaSeconds :type "Float (single-precision)"))
  (`self.colision_for_ball` DeltaSeconds))

(fn `colision_for_ball`
  (params (A :type "Float (single-precision)"))
  (if (> (`self.speed`) (`self.minimumSpeed`))
    (bind _output_get (set `self.speed` (- (`self.speed`) (`self.StopSpeed`)))))
  (bind _sweephitresult (`self.K2_AddActorWorldOffset` (* A (* _output_get (`self.poss`))) true))
  (bind (_bblockinghit _binitialoverlap _time _distance _location _impactpoint _normal) (`GameplayStatics.BreakHitResult` _sweephitresult))
  (if _bblockinghit
    (set `self.poss` (`KismetMathLibrary.GetReflectionVector` (`self.poss`) _normal))))

(fn `UserConstructionScript`)