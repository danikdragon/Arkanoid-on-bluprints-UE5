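; BP_destructeble is an actor that takes damage when a BP_movementBall overlaps it and eventually destroys itself.
; Each ball overlap subtracts DamageOnOneHIt from Heals while Heals differs from HealsForDestr.
; An overlap that finds the two equal destroys the actor, so destruction takes one hit after reaching the threshold.
; The test is exact equality, so damage that steps past HealsForDestr never triggers destruction.
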(event `self.ReceiveActorBeginOverlap`
  (params (OtherActor :type "Actor Object Reference"))
  (cast `/Game/MiActor/6/BP_movementBall` OtherActor)
  (if (!= (`self.Heals`) (`self.HealsForDestr`))
    (set `self.Heals` (- (`self.Heals`) (`self.damageOnOneHIt`)))
    (else
      (`self.K2_DestroyActor`)
      (if (!= (`self.Heals`) (`self.HealsForDestr`))
        _))))

(fn `UserConstructionScript`)